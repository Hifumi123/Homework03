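; AI controller for the zombie that runs BT_Zombie on possess and feeds its Blackboard with the player target.
; Sensing a Player-tagged actor sets HasLineOfSight and PlayerActor and cancels the forget timer.
; Any other perception update starts that timer, which clears both keys after LineOfSightTimer expires.
; AfterBeHit bypasses perception by writing the Hitter as the visible target.
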(event `self.ReceivePossess`
  (params (PossessedPawn :type "Pawn Object Reference"))
  (`self.RunBehaviorTree` "/Game/Work/AI/Zombie/BT_Zombie.BT_Zombie"))

(event `self.AIPerception.OnTargetPerceptionUpdated`
  (params (Actor :type "Actor Object Reference") (Stimulus :type "AIStimulus Structure"))
  (bind _blackboard (`self.Blackboard`))
  (if (and (`self.ActorHasTag` Actor "Player") (`.bSuccessfullySensed` (break `AIStimulus` Stimulus)))
    (`KismetSystemLibrary.K2_ClearAndInvalidateTimerHandle` (`self.EnemyTimer`))
    (`BlackboardComponent.SetValueAsBool` _blackboard (`self.HasLineOfSight`) true)
    (`BlackboardComponent.SetValueAsObject` _blackboard (`self.PlayerActor`) Actor)
    (else
      (bind _returnvalue (`KismetSystemLibrary.K2_SetTimerDelegate` (delegate `StartEnemyTimer`) (`self.LineOfSightTimer`)))
      (set `self.EnemyTimer` _returnvalue))))

(event `StartEnemyTimer`
  (bind _blackboard (`self.Blackboard`))
  (`BlackboardComponent.SetValueAsBool` _blackboard (`self.HasLineOfSight`) false)
  (`BlackboardComponent.SetValueAsObject` _blackboard (`self.PlayerActor`) null))

(fn `AfterBeHit`
  (params (Hitter :type "Actor Object Reference"))
  (bind _blackboard (`self.Blackboard`))
  (`BlackboardComponent.SetValueAsBool` _blackboard (`self.HasLineOfSight`) true)
  (`BlackboardComponent.SetValueAsObject` _blackboard (`self.PlayerActor`) Hitter))

(fn `UserConstructionScript`)