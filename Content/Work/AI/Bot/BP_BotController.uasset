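; BP_BotController is the AI controller for bots, running BT_Bot on possession and feeding it target data through the blackboard.
; Perception updates for Player-tagged actors set HasLineOfSight and TargetActor when sensed.
; On losing sight it clears line of sight at once but starts an 8-second timer, cancelled on re-detection, before clearing the target.
; AfterBeHit makes the attacker the visible target, bypassing perception.
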(event `self.ReceivePossess`
  (params (PossessedPawn :type "Pawn Object Reference"))
  (`self.RunBehaviorTree` "/Game/Work/AI/Bot/BT_Bot.BT_Bot"))

(event `self.AIPerception.OnTargetPerceptionUpdated`
  (params (Actor :type "Actor Object Reference") (Stimulus :type "AIStimulus Structure"))
  (set `self.PerceivedActor` Actor)
  (if (`self.ActorHasTag` Actor "Player")
    (if (`.bSuccessfullySensed` (break `AIStimulus` Stimulus))
      (`KismetSystemLibrary.K2_ClearAndInvalidateTimerHandle` (`self.LostSightTimer`))
      (`self.UpdateSightKey` true)
      (`self.UpdateTargetKey` (`self.PerceivedActor`))
      (else
        (bind _returnvalue (`KismetSystemLibrary.K2_SetTimerDelegate` (delegate `LostSight`) 8.0))
        (set `self.LostSightTimer` _returnvalue)
        (`self.UpdateSightKey` false)))))

(event `LostSight`
  (`self.UpdateTargetKey` null))

(fn `AfterBeHit`
  (params (Hitter :type "Actor Object Reference"))
  (`self.UpdateSightKey` true)
  (`self.UpdateTargetKey` Hitter))

(fn `UpdateSightKey`
  (params (HasLineOfSight :type Boolean))
  (`BlackboardComponent.SetValueAsBool` (`self.Blackboard`) "HasLineOfSight" HasLineOfSight))

(fn `UpdateTargetKey`
  (params (TargetActor :type "Actor Object Reference"))
  (`BlackboardComponent.SetValueAsObject` (`self.Blackboard`) "TargetActor" TargetActor))

(fn `UserConstructionScript`)