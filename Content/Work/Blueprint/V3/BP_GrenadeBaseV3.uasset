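; Base grenade actor that launches its mesh along the player controller's aim and detonates after a delay.
; Detonation spawns an isolated or attached particle emitter plus a sound, calls the empty CauseDamage hook, then hides the mesh.
; After a set duration, DestroyAll removes the stored emitter and sound, destroying the actor only when both exist; the attached emitter's reference is never stored.
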(event `self.ReceiveBeginPlay`
  (bind _staticmesh (`self.StaticMesh`))
  (bind _emittertemplate (`self.EmitterTemplate`))
  (bind _emitterscale (`self.EmitterScale`))
  (bind _returnvalue (`SceneComponent.K2_GetComponentLocation` _staticmesh))
  (`PrimitiveComponent.AddImpulse` _staticmesh (* (`KismetMathLibrary.Conv_RotatorToVector` (`Controller.GetControlRotation` (`GameplayStatics.GetPlayerController` 0))) (* (`self.ImpulseDirection`) (`self.ImpulseValue`))) "None" false)
  (`KismetSystemLibrary.Delay` (`self.Delay`))
  (if (`self.EmitterIsIsolated`)
    (bind _returnvalue_2 (`GameplayStatics.SpawnEmitterAtLocation` _emittertemplate _returnvalue (struct) _emitterscale false))
    (else
      (`GameplayStatics.SpawnEmitterAttached` _emittertemplate _staticmesh "None" (0.0 0.0 0.0) (struct) _emitterscale "KeepRelativeOffset" false)))
  (bind _returnvalue_3 (`GameplayStatics.SpawnSoundAtLocation` (`self.Sound`) _returnvalue (struct) 1.0 1.0 0.0 null null false))
  (`self.CauseDamage`)
  (`SceneComponent.SetVisibility` (`self.StaticMesh`) false false)
  (`KismetSystemLibrary.Delay` (`self.Duration`))
  (`self.DestroyAll` _returnvalue_2 _returnvalue_3))

(fn `CauseDamage`)

(fn `DestroyAll`
  (params (Emitter :type "ParticleSystemComponent Object Reference") (Sound :type "AudioComponent Object Reference"))
  (bind _result (`self.IsNull` Emitter))
  (if (not _result)
    (`ActorComponent.K2_DestroyComponent` Emitter)
    (bind _result_2 (`self.IsNull` Sound))
    (if (not _result_2)
      (`ActorComponent.K2_DestroyComponent` Sound)
      (`self.K2_DestroyActor`))))

(fn `IsNull`
  (params (Actor :type "ActorComponent Object Reference"))
  (returns (Result :type Boolean))
  (return (== Actor null)))

(fn `UserConstructionScript`)