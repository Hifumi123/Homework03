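; Player-controlled FPS character that maps input actions to movement, combat and HUD behavior, building on parent-class logic.
; Sprint, crouch and aim-down-sights adjust walk speed and interrupt one another, with ADS switching cameras.
; Fire repeats on the equipped weapon's fire-rate delay; input also drives reloading, primary/secondary swapping and grenades.
; Player 0 gets a HUD and velocity-driven crosshair spread, while TakeDamage adds a damage-effect widget.
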(event `self.ReceiveBeginPlay`
  (`parent.ReceiveBeginPlay`)
  (bind _result (`self.IsPlayer0`))
  (if _result
    (bind _returnvalue (`|CreateWidget` "/Game/Work/Blueprint/V3/WBP_FPSHUDv3.WBP_FPSHUDv3_C"))
    (`UserWidget.AddToViewport` _returnvalue 0)
    (bind _returnvalue_2 (`|CreateWidget` "/Game/Work/Blueprint/V3/WBP_CrosshairV3.WBP_CrosshairV3_C"))
    (bind _output_get (set `self.L_Crosshair` _returnvalue_2))
    (`UserWidget.AddToViewport` _output_get 0)))

(event `self.ReceiveTick`
  (params (DeltaSeconds :type "Float (single-precision)"))
  (`parent.ReceiveTick` DeltaSeconds)
  (bind _result (`self.IsPlayer0`))
  (if _result
    (set `/Game/Work/Blueprint/V3/WBP_CrosshairV3.crosshair_spread` (`KismetMathLibrary.MapRangeClamped` (`KismetMathLibrary.VSize` (`self.GetVelocity`)) 0.0 450.0 5.0 80.0) (`self.L_Crosshair`))))

(event `InputAction|Fire`
  (params (Key :type "Key Structure"))
  (:`Pressed`
    (if (not (or (`self.SprintTrue`) (`self.IsReloading`))) :!label _label
      (`self.Fire`)
      (`KismetSystemLibrary.Delay` (`/Game/Work/Blueprint/V3/BP_WeaponBaseV3.FireRate` (`self.EquippedWeapon`)))
      (if (`self.IsFiring`)
        (goto _label))))
  (:`Released`
    (set `self.IsFiring` false)))

(event `InputAction|Crouch`
  (params (Key :type "Key Structure"))
  (:`Pressed`
    (if (`self.SprintTrue`)
      (set `self.SprintTrue` false))
    (set `self.CrouchTrue` true)
    (set `CharacterMovementComponent.MaxWalkSpeed` 300.0 (`self.CharacterMovement`))
    (`self.Crouch`))
  (:`Released`
    (set `self.CrouchTrue` false)
    (set `CharacterMovementComponent.MaxWalkSpeed` 600.0 (`self.CharacterMovement`))
    (`self.UnCrouch`)))

(event `InputAction|Sprint`
  (params (Key :type "Key Structure"))
  (:`Pressed`
    (if (`self.IsAiming`)
      (`self.DeactivateADS`))
    (if (`self.CrouchTrue`)
      (set `self.CrouchTrue` false)
      (`self.UnCrouch`))
    (set `self.SprintTrue` true)
    (set `CharacterMovementComponent.MaxWalkSpeed` 1000.0 (`self.CharacterMovement`)))
  (:`Released`
    (set `self.SprintTrue` false)
    (set `CharacterMovementComponent.MaxWalkSpeed` 600.0 (`self.CharacterMovement`))))

(event `InputAction|AimDownSight`
  (params (Key :type "Key Structure"))
  (:`Pressed`
    (if (not (`self.IsReloading`))
      (if (`self.SprintTrue`)
        (set `self.SprintTrue` false)
        (set `CharacterMovementComponent.MaxWalkSpeed` 600.0 (`self.CharacterMovement`)))
      (`self.SetCurrentCamera` (`self.ADSCamera`) (`self.FollowCamera`))
      (set `CharacterMovementComponent.MaxWalkSpeed` 300.0 (`self.CharacterMovement`))
      (set `self.IsAiming` true)))
  (:`Released`
    (`self.DeactivateADS`)))

(event `InputAction|Reload`
  (params (Key :type "Key Structure"))
  (:`Pressed`
    (`self.Reload`)
    (if (`self.IsReloading`)
      (`KismetSystemLibrary.Delay` 3.3)
      (set `self.IsReloading` false))))

(event `InputAction|SelectPrimary`
  (params (Key :type "Key Structure"))
  (:`Pressed`
    (set `self.EquippedWeapon` (`self.PrimaryWeapon`))
    (`self.SetWeaponVisibility` (`self.SecondaryWeapon`))
    (`self.SetWeaponVisibility` (`self.PrimaryWeapon`) true)
    (`self.SetADSCameraTransform`)))

(event `InputAction|SelectSecondary`
  (params (Key :type "Key Structure"))
  (:`Pressed`
    (if (`self.HaveSecondaryWeapon`)
      (set `self.EquippedWeapon` (`self.SecondaryWeapon`))
      (`self.SetWeaponVisibility` (`self.SecondaryWeapon`) true)
      (`self.SetWeaponVisibility` (`self.PrimaryWeapon`))
      (`self.SetADSCameraTransform`))))

(event `InputAction|FragGrenade`
  (params (Key :type "Key Structure"))
  (:`Pressed`
    (`self.UseGrenade` (`self.FragGrenade`) "/Game/Work/Blueprint/V3/BP_FragGrenadeV3.BP_FragGrenadeV3_C")))

(event `InputAction|SmokeGrenade`
  (params (Key :type "Key Structure"))
  (:`Pressed`
    (`self.UseGrenade` (`self.SmokeGrenade`) "/Game/Work/Blueprint/V3/BP_SmokeGrenadeV3.BP_SmokeGrenadeV3_C")))

(fn `TakeDamage`
  (params (Damage :type "Float (double-precision)") (Hitter :type "Actor Object Reference"))
  (`parent.TakeDamage` Damage Hitter)
  (bind _returnvalue (`|CreateWidget` "/Game/Work/Blueprint/V3/WBP_DamageEffectV3.WBP_DamageEffectV3_C"))
  (`UserWidget.AddToViewport` _returnvalue 0))

(fn `UserConstructionScript`
  (`parent.UserConstructionScript`))