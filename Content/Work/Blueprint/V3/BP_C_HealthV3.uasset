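; Health component Blueprint that tracks Health and a regenerating Armor pool that absorbs damage first.
; TakeDamage subtracts from Armor, carries any overflow into Health and clamps Armor at zero.
; Tick runs through a Delay to add ArmorRecover about once per second, capping Armor at full, while Health does not regenerate.
; IsDead reports whether Health has reached zero or below.
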(event `self.ReceiveTick`
  (params (DeltaSeconds :type "Float (single-precision)"))
  (`KismetSystemLibrary.Delay` 1.0)
  (if (< (`self.Armor`) 1.0)
    (bind _output_get (set `self.L_Health` (+ (`self.Armor`) (`self.ArmorRecover`))))
    (if (> _output_get 1.0)
      (set `self.L_Health` 1.0))
    (set `self.Armor` (`self.L_Health`))))

(fn `IsDead`
  (returns (Result :type Boolean))
  (return (<= (`self.Health`) 0.0)))

(fn `TakeDamage`
  (params (Damage :type "Float (double-precision)"))
  (bind _output_get (set `self.Armor` (- (`self.Armor`) Damage)))
  (if (< _output_get 0.0)
    (set `self.Health` (+ (`self.Health`) (`self.Armor`)))
    (set `self.Armor` 0.0)))