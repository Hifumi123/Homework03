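; BP_BotCharacterV3 is an AI bot character that extends its parent's damage handling with death and hit-reaction logic.
; TakeDamage runs the parent implementation, then asks the BPCHealthV3 component whether the bot is dead.
; A dead bot calls DestroyAll, while a surviving one passes the hitter to BP_BotController through AfterBeHit.
; The event graph holds only disabled default events.
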(fn `TakeDamage`
  (params (Damage :type "Float (double-precision)") (Hitter :type "Actor Object Reference"))
  (`parent.TakeDamage` Damage Hitter)
  (bind _result (`/Game/Work/Blueprint/V3/BP_C_HealthV3.IsDead` (`self.BP_C_HealthV3`)))
  (if _result
    (`self.DestroyAll`)
    (else
      (bind _asbp_bot_controller (cast `/Game/Work/AI/Bot/BP_BotController` (`AIBlueprintHelperLibrary.GetAIController` self)))
      (`/Game/Work/AI/Bot/BP_BotController.AfterBeHit` _asbp_bot_controller Hitter))))

(fn `UserConstructionScript`
  (`parent.UserConstructionScript`))