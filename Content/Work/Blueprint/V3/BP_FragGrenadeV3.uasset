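; Frag grenade Blueprint that deals blast damage to zombies, built on a parent class that supplies the base grenade behavior.
; It overrides CauseDamage to run the parent logic, then gathers the actors overlapping its Sphere component and casts them to BP_ZombieCharacterV3, calling BeBoom with the Damage value on those that match.
; The event graph holds only disabled placeholder events.
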(fn `CauseDamage`
  (`parent.CauseDamage`)
  (for _array_element (`PrimitiveComponent.GetOverlappingActors` (`self.Sphere`) null)
    (bind _asbp_zombie_character_v3 (cast `/Game/Work/Blueprint/V3/BP_ZombieCharacterV3` _array_element))
    (`/Game/Work/Blueprint/V3/BP_ZombieCharacterV3.BeBoom` _asbp_zombie_character_v3 (`self.Damage`))))

(fn `UserConstructionScript`
  (`parent.UserConstructionScript`))