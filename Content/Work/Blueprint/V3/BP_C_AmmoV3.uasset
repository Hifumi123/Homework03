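; Ammo component that tracks a clip and its reserve pool for firing and reloading.
; Fire removes one round while Ammo is above zero, and CanFire reports whether any remain.
; Reload tops the clip up to ClipSize from MaxAmmo, or takes the whole reserve when it is too small.
; CanReload only checks that the clip is below ClipSize, ignoring the reserve; the event graph is unused.
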(fn `CanFire`
  (returns (Result :type Boolean))
  (return (> (`self.Ammo`) 0)))

(fn `CanReload`
  (returns (Result :type Boolean))
  (return (< (`self.Ammo`) (`self.ClipSize`))))

(fn `Fire`
  (if (> (`self.Ammo`) 0)
    (`/Engine/EditorBlueprintResources/StandardMacros.DecrementInt` (`self.Ammo`))))

(fn `Reload`
  (bind _returnvalue (- (`self.ClipSize`) (`self.Ammo`)))
  (if (< (`self.Ammo`) (`self.ClipSize`))
    (if (> (`self.MaxAmmo`) _returnvalue)
      (set `self.L_AmmoDifference` _returnvalue)
      (set `self.Ammo` (+ (`self.Ammo`) (`self.L_AmmoDifference`)))
      (set `self.MaxAmmo` (- (`self.MaxAmmo`) (`self.L_AmmoDifference`)))
      (else
        (set `self.Ammo` (+ (`self.Ammo`) (`self.MaxAmmo`)))
        (set `self.MaxAmmo` 0)))))