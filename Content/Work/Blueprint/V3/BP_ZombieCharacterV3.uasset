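; BP_ZombieCharacterV3 is a zombie enemy that melees the player and takes hit and blast damage.
; While IsAttacking, sphere overlaps damage the player, guarded by AlreadyHit.
; BeHit and BeBoom feed BPCHealthV3, destroying the zombie with a kill popup on death.
; BeHit also shows a hit marker and, on survival, spawns an explosion effect and passes the hitter to BP_ZombieController.
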(event `self.ReceiveActorBeginOverlap`
  (params (OtherActor :type "Actor Object Reference")))

(event `self.Sphere.OnComponentBeginOverlap`
  (params (OverlappedComponent :type "PrimitiveComponent Object Reference") (OtherActor :type "Actor Object Reference") (OtherComp :type "PrimitiveComponent Object Reference") (OtherBodyIndex :type Integer) (bFromSweep :type Boolean) (SweepResult :type "HitResult Structure (by ref)"))
  (bind _asbp_player_character_base_v3 (cast `/Game/Work/Blueprint/V3/BP_PlayerCharacterBaseV3` OtherActor))
  (if (`self.IsAttacking`)
    (if (not (`self.AlreadyHit`))
      (`/Game/Work/Blueprint/V3/BP_PlayerCharacterBaseV3.TakeDamage` _asbp_player_character_base_v3 (`self.Damage`) null)
      (set `self.AlreadyHit` true))))

(fn `BeBoom`
  (params (Damage :type "Float (double-precision)"))
  (bind _bp_c_healthv3 (`self.BP_C_HealthV3`))
  (`/Game/Work/Blueprint/V3/BP_C_HealthV3.TakeDamage` _bp_c_healthv3 Damage)
  (bind _result (`/Game/Work/Blueprint/V3/BP_C_HealthV3.IsDead` _bp_c_healthv3))
  (if _result
    (`self.K2_DestroyActor`)
    (bind _returnvalue (`|CreateWidget` "/Game/Work/Blueprint/V3/WBP_KillPopupV3.WBP_KillPopupV3_C"))
    (`UserWidget.AddToViewport` _returnvalue 0)))

(fn `BeHit`
  (params (Damage :type "Float (double-precision)") (Location :type "Vector Structure") (Hitter :type "Actor Object Reference"))
  (bind _bp_c_healthv3 (`self.BP_C_HealthV3`))
  (bind _returnvalue (`|CreateWidget` "/Game/Work/Blueprint/V3/WBP_HitMarkerV3.WBP_HitMarkerV3_C"))
  (`UserWidget.AddToViewport` _returnvalue 0)
  (`/Game/Work/Blueprint/V3/BP_C_HealthV3.TakeDamage` _bp_c_healthv3 Damage)
  (bind _result (`/Game/Work/Blueprint/V3/BP_C_HealthV3.IsDead` _bp_c_healthv3))
  (if _result
    (`self.K2_DestroyActor`)
    (bind _returnvalue_2 (`|CreateWidget` "/Game/Work/Blueprint/V3/WBP_KillPopupV3.WBP_KillPopupV3_C"))
    (`UserWidget.AddToViewport` _returnvalue_2 0)
    (else
      (`GameplayStatics.SpawnEmitterAtLocation` "/Game/StarterContent/Particles/P_Explosion.P_Explosion" Location)
      (bind _asbp_zombie_controller (cast `/Game/Work/AI/Zombie/BP_ZombieController` (`AIBlueprintHelperLibrary.GetAIController` self)))
      (`/Game/Work/AI/Zombie/BP_ZombieController.AfterBeHit` _asbp_zombie_controller Hitter))))

(fn `UpdateWalkSpeed`
  (params (NewWalkSpeed :type "Float (double-precision)"))
  (set `CharacterMovementComponent.MaxWalkSpeed` NewWalkSpeed (`self.CharacterMovement`)))

(fn `UserConstructionScript`)