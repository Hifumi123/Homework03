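; Base weapon actor providing hitscan firing and reloading for player characters.
; Fire line-traces on Visibility from the ADS or follow camera, depending on aim state, out to Range, damaging zombies via BeHit or players via TakeDamage.
; It then updates the ammo component and spawns flash and sound at the Muzzle socket.
; Fire/reload checks and reloading delegate to the ammo component.
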(fn `CanFire`
  (returns (Result :type Boolean))
  (bind _result (`/Game/Work/Blueprint/V3/BP_C_AmmoV3.CanFire` (`self.BP_C_AmmoV3`)))
  (return _result))

(fn `CanReload`
  (returns (Result :type Boolean))
  (bind _result (`/Game/Work/Blueprint/V3/BP_C_AmmoV3.CanReload` (`self.BP_C_AmmoV3`)))
  (return _result))

(fn `Fire`
  (params (BP_PlayerCharacterBaseV3 :type "/Game/Work/Blueprint/V3/BP_PlayerCharacterBaseV3 Object Reference"))
  (bind _skeletalmesh (`self.SkeletalMesh`))
  (bind _returnvalue (`SceneComponent.GetSocketLocation` _skeletalmesh "Muzzle"))
  (`self.LineTrace` BP_PlayerCharacterBaseV3)
  (`/Game/Work/Blueprint/V3/BP_C_AmmoV3.Fire` (`self.BP_C_AmmoV3`))
  (bind _returnvalue_2 (`GameplayStatics.SpawnEmitterAtLocation` "/Game/InfinityBladeEffects/Effects/FX_Monsters/FX_Monster_Chicken/P_ChickenMaster_MuzzleFlash_01.P_ChickenMaster_MuzzleFlash_01" _returnvalue (`SceneComponent.GetSocketRotation` _skeletalmesh "Muzzle")))
  (`SceneComponent.SetWorldScale3D` _returnvalue_2 (0.1 0.1 0.1))
  (`GameplayStatics.SpawnSoundAtLocation` "/Game/StarterContent/Audio/Explosion01.Explosion01" _returnvalue (struct) 1.0 1.0 0.0 null null))

(fn `L_GetLinePoints`
  (params (Camera :type "CameraComponent Object Reference"))
  (returns (Start :type "Vector Structure") (End :type "Vector Structure"))
  (bind _returnvalue (`SceneComponent.K2_GetComponentLocation` Camera))
  (return _returnvalue (+ _returnvalue (* (`KismetMathLibrary.GetForwardVector` (`SceneComponent.K2_GetComponentRotation` Camera)) (`self.Range`)))))

(fn `LineTrace`
  (params (BP_PlayerCharacterBaseV3 :type "/Game/Work/Blueprint/V3/BP_PlayerCharacterBaseV3 Object Reference"))
  (if (`/Game/Work/Blueprint/V3/BP_PlayerCharacterBaseV3.IsAiming` BP_PlayerCharacterBaseV3)
    (bind (_start _end) (`self.L_GetLinePoints` (`/Game/Work/Blueprint/V3/BP_PlayerCharacterBaseV3.ADSCamera` BP_PlayerCharacterBaseV3)))
    (bind _outhit (`KismetSystemLibrary.LineTraceSingle` _start _end "TraceTypeQuery1" false (`|MakeArray` BP_PlayerCharacterBaseV3 :!type "Actor Object Reference")))
    (bind (_bblockinghit _binitialoverlap _time _distance _location _impactpoint _normal _impactnormal _physmat _hitactor) (`GameplayStatics.BreakHitResult` _outhit))
    (bind _asbp_zombie_character_v3 (cast `/Game/Work/Blueprint/V3/BP_ZombieCharacterV3` _hitactor)
      (:`then`
        (`/Game/Work/Blueprint/V3/BP_ZombieCharacterV3.BeHit` _asbp_zombie_character_v3 (`self.Damage`) _location BP_PlayerCharacterBaseV3))
      (:`CastFailed`
        (bind _asbp_player_character_base_v3 (cast `/Game/Work/Blueprint/V3/BP_PlayerCharacterBaseV3` _hitactor))
        (`/Game/Work/Blueprint/V3/BP_PlayerCharacterBaseV3.TakeDamage` _asbp_player_character_base_v3 (`self.Damage`) BP_PlayerCharacterBaseV3)))
    (else
      (bind (_start_2 _end_2) (`self.L_GetLinePoints` (`/Game/Work/Blueprint/V3/BP_PlayerCharacterBaseV3.FollowCamera` BP_PlayerCharacterBaseV3)))
      (bind _outhit_2 (`KismetSystemLibrary.LineTraceSingle` _start_2 _end_2 "TraceTypeQuery1" false (`|MakeArray` BP_PlayerCharacterBaseV3 :!type "Actor Object Reference")))
      (bind (_bblockinghit_2 _binitialoverlap_2 _time_2 _distance_2 _location_2 _impactpoint_2 _normal_2 _impactnormal_2 _physmat_2 _hitactor_2) (`GameplayStatics.BreakHitResult` _outhit_2))
      (bind _asbp_zombie_character_v3_2 (cast `/Game/Work/Blueprint/V3/BP_ZombieCharacterV3` _hitactor_2)
        (:`then`
          (`/Game/Work/Blueprint/V3/BP_ZombieCharacterV3.BeHit` _asbp_zombie_character_v3_2 (`self.Damage`) _location_2 BP_PlayerCharacterBaseV3))
        (:`CastFailed`
          (bind _asbp_player_character_base_v3_2 (cast `/Game/Work/Blueprint/V3/BP_PlayerCharacterBaseV3` _hitactor_2))
          (`/Game/Work/Blueprint/V3/BP_PlayerCharacterBaseV3.TakeDamage` _asbp_player_character_base_v3_2 (`self.Damage`) BP_PlayerCharacterBaseV3))))))

(fn `Reload`
  (`/Game/Work/Blueprint/V3/BP_C_AmmoV3.Reload` (`self.BP_C_AmmoV3`)))

(fn `UserConstructionScript`)