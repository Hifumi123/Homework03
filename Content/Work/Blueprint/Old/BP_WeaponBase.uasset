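; Base weapon Blueprint for the player character, providing hitscan firing and magazine reloading.
; Fire traces from the ADS or follow camera by aim state, calls BeHit on SimpleAI hits, decrements Ammo unchecked and spawns a muzzle flash at the equipped weapon's socket.
; Reload tops up the clip from MaxAmmo reserves and sets the player's IsReloading flag.
; Traces draw persistent debug lines; a disconnected projectile-firing chain and older reload function remain.
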(event `Fire`
  (bind _asbp_player_character (cast `/Game/Work/Blueprint/Old/BP_PlayerCharacter` (`GameplayStatics.GetPlayerCharacter` 0)))
  (`self.LineTrace` _asbp_player_character)
  (set `self.Ammo` (- (`self.Ammo`) 1))
  (bind _asbp_player_character_2 (cast `/Game/Work/Blueprint/Old/BP_PlayerCharacter` (`GameplayStatics.GetPlayerCharacter` 0)))
  (bind _skeletalmesh (`/Game/Work/Blueprint/Old/BP_WeaponBase.SkeletalMesh` (`/Game/Work/Blueprint/Old/BP_PlayerCharacter.EquippedWeapon` _asbp_player_character_2)))
  (bind _returnvalue (`GameplayStatics.SpawnEmitterAtLocation` "/Game/InfinityBladeEffects/Effects/FX_Monsters/FX_Monster_Chicken/P_ChickenMaster_MuzzleFlash_01.P_ChickenMaster_MuzzleFlash_01" (`SceneComponent.GetSocketLocation` _skeletalmesh "Muzzle") (`SceneComponent.GetSocketRotation` _skeletalmesh "Muzzle")))
  (`SceneComponent.SetWorldScale3D` _returnvalue (0.1 0.1 0.1)))

(fn `LineTrace`
  (params (BP_PlayerCharacter :type "/Game/Work/Blueprint/Old/BP_PlayerCharacter Object Reference"))
  (bind _bp_playercharacter (`local.BP_PlayerCharacter`))
  (bind _adscamera (`/Game/Work/Blueprint/Old/BP_PlayerCharacter.ADSCamera` _bp_playercharacter))
  (bind _followcamera (`/Game/Work/Blueprint/Old/BP_PlayerCharacter.FollowCamera` _bp_playercharacter))
  (bind _returnvalue (`SceneComponent.K2_GetComponentLocation` _adscamera))
  (bind _returnvalue_2 (`SceneComponent.K2_GetComponentLocation` _followcamera))
  (if (`/Game/Work/Blueprint/Old/BP_PlayerCharacter.IsAiming` _bp_playercharacter)
    (bind _outhit (`KismetSystemLibrary.LineTraceSingle` :`Start` _returnvalue :`End` (+ _returnvalue (* (`KismetMathLibrary.GetForwardVector` (`SceneComponent.K2_GetComponentRotation` _adscamera)) 1500.0)) :`TraceChannel` "TraceTypeQuery1" :`DrawDebugType` "Persistent"))
    (bind (_bblockinghit _binitialoverlap _time _distance _location _impactpoint _normal _impactnormal _physmat _hitactor) (`GameplayStatics.BreakHitResult` _outhit))
    (bind _assimple_ai (cast `/Game/Work/Blueprint/Old/SimpleAI` _hitactor))
    (`/Game/Work/Blueprint/Old/SimpleAI.BeHit` _assimple_ai _location)
    (else
      (bind _outhit_2 (`KismetSystemLibrary.LineTraceSingle` :`Start` _returnvalue_2 :`End` (+ _returnvalue_2 (* (`KismetMathLibrary.GetForwardVector` (`SceneComponent.K2_GetComponentRotation` _followcamera)) 1500.0)) :`TraceChannel` "TraceTypeQuery1" :`DrawDebugType` "Persistent"))
      (bind (_bblockinghit_2 _binitialoverlap_2 _time_2 _distance_2 _location_2 _impactpoint_2 _normal_2 _impactnormal_2 _physmat_2 _hitactor_2) (`GameplayStatics.BreakHitResult` _outhit_2))
      (bind _assimple_ai_2 (cast `/Game/Work/Blueprint/Old/SimpleAI` _hitactor_2))
      (`/Game/Work/Blueprint/Old/SimpleAI.BeHit` _assimple_ai_2 _location_2))))

(fn `Reload`
  (returns (IsReloading :type Boolean))
  (bind _returnvalue (- (`self.ClipSize`) (`self.Ammo`)))
  (if (< (`self.Ammo`) (`self.ClipSize`))
    (if (> (`self.MaxAmmo`) _returnvalue)
      (set `self.AmmoDifference` _returnvalue)
      (set `self.Ammo` (+ (`self.Ammo`) (`self.AmmoDifference`)))
      (set `self.MaxAmmo` (- (`self.MaxAmmo`) (`self.AmmoDifference`)))
      (bind _asbp_player_character (cast `/Game/Work/Blueprint/Old/BP_PlayerCharacter` (`GameplayStatics.GetPlayerCharacter` 0)))
      (set `/Game/Work/Blueprint/Old/BP_PlayerCharacter.IsReloading` true _asbp_player_character)
      (else
        (set `self.AmmoDifference` _returnvalue)
        (set `self.Ammo` (+ (`self.Ammo`) (`self.MaxAmmo`)))
        (set `self.MaxAmmo` 0)
        (bind _asbp_player_character_2 (cast `/Game/Work/Blueprint/Old/BP_PlayerCharacter` (`GameplayStatics.GetPlayerCharacter` 0)))
        (set `/Game/Work/Blueprint/Old/BP_PlayerCharacter.IsReloading` true _asbp_player_character_2)))
    (return true)
    (else
      (`KismetSystemLibrary.PrintString` "Full Ammo"))))

(fn `Reload_Old`
  (if (== (`self.Ammo`) (`self.ClipSize`))
    _
    (elif (> (`self.MaxAmmo`) (`self.ClipSize`))
      (set `self.Ammo` (`self.ClipSize`))
      (set `self.MaxAmmo` (- (`self.MaxAmmo`) (`self.Ammo`)))
      (else
        (set `self.Ammo` (`self.MaxAmmo`))
        (set `self.MaxAmmo` 0)))))

(fn `UserConstructionScript`)