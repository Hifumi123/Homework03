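; M4A1 weapon Blueprint that handles firing and reloading.
; Fire spawns a projectile at its Muzzle socket and decrements Ammo without checking it, then places a scaled-down muzzle flash on the player's SecondaryWeapon rather than itself.
; Reload tops up the clip from MaxAmmo and sets the player's IsReloading flag, or prints when full.
; ReloadOld is an alternate refill without that flag.
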(event `Fire`
  (`|SpawnActorFromClass` "/Game/Work/Blueprint/Old/BP_ProjectileBase.BP_ProjectileBase_C" (`SceneComponent.GetSocketTransform` (`self.SkeletalMesh`) "Muzzle" "RTS_World") "Undefined" "OverrideRootScale" null null)
  (set `self.Ammo` (- (`self.Ammo`) 1))
  (bind _asbp_player_character (cast `/Game/Work/Blueprint/Old/BP_PlayerCharacter` (`GameplayStatics.GetPlayerCharacter` 0)))
  (bind _skeletalmesh (`/Game/Work/Blueprint/Old/BP_Weapon_M4A1.SkeletalMesh` (`/Game/Work/Blueprint/Old/BP_PlayerCharacter.SecondaryWeapon` _asbp_player_character)))
  (bind _returnvalue (`GameplayStatics.SpawnEmitterAtLocation` "/Game/InfinityBladeEffects/Effects/FX_Monsters/FX_Monster_Chicken/P_ChickenMaster_MuzzleFlash_01.P_ChickenMaster_MuzzleFlash_01" (`SceneComponent.GetSocketLocation` _skeletalmesh "Muzzle") (`SceneComponent.GetSocketRotation` _skeletalmesh "Muzzle")))
  (`SceneComponent.SetWorldScale3D` _returnvalue (0.1 0.1 0.1)))

(fn `Reload`
  (returns (IsReloading :type Boolean))
  (bind _returnvalue (- (`self.ClipSize`) (`self.Ammo`)))
  (if (< (`self.Ammo`) (`self.ClipSize`))
    (if (> (`self.MaxAmmo`) _returnvalue)
      (set `self.AmmoDifference` _returnvalue)
      (set `self.Ammo` (+ (`self.Ammo`) (`self.AmmoDifference`)))
      (set `self.MaxAmmo` (- (`self.MaxAmmo`) (`self.AmmoDifference`)))
      (bind _asbp_player_character (cast `/Game/Work/Blueprint/Old/BP_PlayerCharacter` (`GameplayStatics.GetPlayerCharacter` 0)))
      (set `/Game/Work/Blueprint/Old/BP_PlayerCharacter.IsReloading` true _asbp_player_character)
      (else
        (set `self.AmmoDifference` _returnvalue)
        (set `self.Ammo` (+ (`self.Ammo`) (`self.MaxAmmo`)))
        (set `self.MaxAmmo` 0)
        (bind _asbp_player_character_2 (cast `/Game/Work/Blueprint/Old/BP_PlayerCharacter` (`GameplayStatics.GetPlayerCharacter` 0)))
        (set `/Game/Work/Blueprint/Old/BP_PlayerCharacter.IsReloading` true _asbp_player_character_2)))
    (return true)
    (else
      (`KismetSystemLibrary.PrintString` "Full Ammo"))))

(fn `Reload_Old`
  (if (== (`self.Ammo`) (`self.ClipSize`))
    _
    (elif (> (`self.MaxAmmo`) (`self.ClipSize`))
      (set `self.Ammo` (`self.ClipSize`))
      (set `self.MaxAmmo` (- (`self.MaxAmmo`) (`self.Ammo`)))
      (else
        (set `self.Ammo` (`self.MaxAmmo`))
        (set `self.MaxAmmo` 0)))))

(fn `UserConstructionScript`)